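; Alien enemy Blueprint that chases the player on sight and otherwise hunts for them.
; Each Tick, PawnSensing plus a line trace choose between chasing, moving to the last seen position, or searching.
; A Knowledge value rises during sight and decays while searching, gating new random search points around the player's actual location.
; Knowledge tiers set SearchRadius, but the random-point query uses a fixed radius.
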(event `self.ReceiveBeginPlay`
  ;[1 1 1] set speed
  (set `CharacterMovementComponent.MaxWalkSpeed` 300.0 (`self.CharacterMovement`))
  ;[1 1 1] Set Knowledge
  (set `self.Knowledge` 100.0)
  (set `self.LastSeenPos` (+ (`SceneComponent.K2_GetComponentLocation` (`self.Head`)) (`self.GetActorForwardVector` self)))
  (set `self.SearchPos` (`self.K2_GetActorLocation` (`self.player`)))
  (set `self.searching` true)
  (set `self.moving` false))

(event `self.ReceiveTick`
  (params (DeltaSeconds :type "Float (single-precision)"))
  (bind _searchpos (`self.SearchPos`))
  (bind _knowledge (`self.Knowledge`))
  (bind _knowledge_2 (`self.Knowledge`))
  (bind _returnvalue (`PawnSensingComponent.GetPeripheralVisionAngle` (`self.PawnSensing`)))
  ;[1 1 1] Draws debug cone
  (set `self.DeltaTime` DeltaSeconds)
  (`KismetSystemLibrary.DrawDebugConeInDegrees` (`SceneComponent.K2_GetComponentLocation` (`self.CapsuleComponent`)) (`self.GetActorForwardVector` self) 200.0 _returnvalue _returnvalue)
  (bind (_outhit _returnvalue_2) (`KismetSystemLibrary.LineTraceSingle` :`Start` (`SceneComponent.K2_GetComponentLocation` (`self.Head`)) :`End` (`SceneComponent.K2_GetComponentLocation` (`/Game/FirstPersonBP/Blueprints/FirstPersonCharacter.FirstPersonCamera` (`self.player`))) :`TraceChannel` "TraceTypeQuery1" :`DrawDebugType` "ForDuration"))
  ;[1 1 1] If Player can be seen
  (if (and (not _returnvalue_2) (`self.player in sight`))
    (set `self.searching` false)
    (`self.MoveToPlayer` self)
    (set `self.LastSeenPos` (`SceneComponent.K2_GetComponentLocation` (`/Game/FirstPersonBP/Blueprints/FirstPersonCharacter.FirstPersonCamera` (`self.player`))))
    (bind _output_get (set `self.Knowledge` (+ (`self.Knowledge`) (* (`self.DeltaTime`) 5.0))))
    (else
      ;[1 1 1] If ai is searching
      (if (`self.searching`)
        (set `self.player in sight` false)
        (`self.MoveToSearchPos` (`self.SearchPos`))
        (`KismetSystemLibrary.PrintString` "")
        (if (> _knowledge_2 0.0)
          (set `self.Knowledge` (- _knowledge_2 (* (`self.DeltaTime`) 3.0)))
          (`KismetSystemLibrary.PrintString` (`KismetStringLibrary.Conv_VectorToString` _searchpos))
          (if (== (`KismetMathLibrary.MakeVector` (.x (`SceneComponent.K2_GetComponentLocation` (`self.Head`))) (.y (`SceneComponent.K2_GetComponentLocation` (`self.Head`)))) (`KismetMathLibrary.MakeVector` (.x _searchpos) (.y _searchpos)) :`ErrorTolerance` 100.0)
            (`KismetSystemLibrary.PrintString` "Creating random point")
            (if (> _knowledge 0.0)
              ;[1 1 1] Bases Search Radius Off of Knowledge
              (set `self.Knowledge` (- _knowledge (* (`self.DeltaTime`) 1.0)))
              (if (>= (`self.Knowledge`) 75.0)
                (set `self.searchRadius` 5000.0)
                (bind _output_get_2 (set `self.SearchPos` (`NavigationSystem.GetRandomReachablePointInRadius` (`SceneComponent.K2_GetComponentLocation` (`/Game/FirstPersonBP/Blueprints/FirstPersonCharacter.FirstPersonCamera` (`self.player`))) 5000.0) :!label _label))
                (`KismetSystemLibrary.PrintString` (`KismetStringLibrary.Conv_VectorToString` _output_get_2))
                (elif (>= (`self.Knowledge`) 50.0)
                  (set `self.searchRadius` 10000.0)
                  (goto _label)
                  (elif (>= (`self.Knowledge`) 25.0)
                    (set `self.searchRadius` 15000.0)
                    (goto _label)
                    (elif (>= (`self.Knowledge`) -5.0)
                      (set `self.searchRadius` 25000.0)
                      (goto _label))))))))
        (else
          (`self.MoveToLastSeen` (`self.LastSeenPos`))
          (if (== (`KismetMathLibrary.MakeVector` (.x (`SceneComponent.K2_GetComponentLocation` (`self.Head`))) (.y (`SceneComponent.K2_GetComponentLocation` (`self.Head`)))) (`KismetMathLibrary.MakeVector` (.x (`self.LastSeenPos`)) (.y (`self.LastSeenPos`))) :`ErrorTolerance` 100.0)
            (set `self.searching` true)))))))

(event `self.PawnSensing.OnSeePawn`
  (params (Pawn :type "Pawn Object Reference"))
  (cast `/Game/FirstPersonBP/Blueprints/FirstPersonCharacter` Pawn)
  (`KismetSystemLibrary.PrintString` "i see you")
  (set `self.player in sight` true))

(event `self.ReceiveHit`
  (params (MyComp :type "PrimitiveComponent Object Reference") (Other :type "Actor Object Reference") (OtherComp :type "PrimitiveComponent Object Reference") (bSelfMoved :type Boolean) (HitLocation :type "Vector Structure") (HitNormal :type "Vector Structure") (NormalImpulse :type "Vector Structure") (Hit :type "HitResult Structure (by ref)"))
  ;[1 1 1] Allows AI to continue moving
  (cast `/Game/FirstPersonBP/Blueprints/FirstPersonCharacter` Other)
  (set `self.moving` false))

(fn `MoveToLastSeen`
  (params (LastPosition :type "Vector Structure"))
  (bind _returnvalue (`AIBlueprintHelperLibrary.GetAIController` self))
  (`NavigationSystem.SimpleMoveToLocation` _returnvalue LastPosition)
  (set `self.searching` false))

(fn `MoveToPlayer`
  (bind _returnvalue (`AIBlueprintHelperLibrary.GetAIController` self))
  (`NavigationSystem.SimpleMoveToActor` _returnvalue (`self.player`)))

(fn `MoveToSearchPos`
  (params (Search :type "Vector Structure"))
  (bind _returnvalue (`AIBlueprintHelperLibrary.GetAIController` self))
  (`NavigationSystem.SimpleMoveToLocation` _returnvalue Search))

(fn `UserConstructionScript`)